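; BP_ColourSwitch is a sphere actor that cycles through a list of colour materials each time a first-person projectile hits it.
; On BeginPlay it applies the editor-chosen material and finds its index in the list, defaulting to yellow if none is set.
; Collider hits from BP_FirstPersonProjectile call SwitchColor, which advances the index with wraparound, applies and stores the new material, and prints a display name.
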(event OnComponentHit(SphereCollider)
  (params (HitComponent :type Primitive%20Component%20Object%20Reference) (OtherActor :type Actor%20Object%20Reference) (OtherComp :type Primitive%20Component%20Object%20Reference) (NormalImpulse :type Vector :default "0, 0, 0") (Hit :type Hit%20Result%20Structure%20%28by%20ref%29))
  (if (== (Utilities|GetClass OtherActor) "/Game/FirstPerson/Blueprints/BP_FirstPersonProjectile.BP_FirstPersonProjectile_C")
    (CallFunction|SwitchColor)))

(event Custom|Switch%20Color
  (Math|Integer|IncrementInt (Variables|Default|GetCurrent%20Colour%20Index)
    (:%20%20
      (if (== (Variables|Default|GetCurrent%20Colour%20Index) (Variables|Default|GetNumber%20of%20Colours))
        (Variables|Default|SetCurrent%20Colour%20Index 0))
      (Rendering|Material|SetMaterial (Variables|Default|GetSphere) 0 (Utilities|Array|Get(acopy) (Variables|Default|GetList%20of%20Colours) (Variables|Default|GetCurrent%20Colour%20Index)))
      (Variables|Default|SetColour (Utilities|Array|Get(acopy) (Variables|Default|GetList%20of%20Colours) (Variables|Default|GetCurrent%20Colour%20Index)))
      (Development|PrintString (Utilities|GetDisplayName 0)))))

(event EventBeginPlay
  ;[1 1 1] Gets and sets number of colours
  (Variables|Default|SetNumber%20of%20Colours (Utilities|Array|Length (Variables|Default|GetList%20of%20Colours)))
  ;[1 1 1] Sets an Initial Material colour specified in editor, if none was selected then set default Yellow
  (Utilities|IsValid (Variables|Default|GetColour)
    (:Is%20Valid
      (Rendering|Material|SetMaterial (Variables|Default|GetSphere) 0 (Variables|Default|GetColour))
      ;[1 1 1] Loops through List of Colours to compare to Initial Colour to set appropriate Current Colour Index
      (for (_array_element _array_index) (Variables|Default|GetList%20of%20Colours)
        (if (== _array_element (Variables|Default|GetColour))
          (Variables|Default|SetCurrent%20Colour%20Index _array_index))))
    (:Is%20Not%20Valid
      (Rendering|Material|SetMaterial (Variables|Default|GetSphere) 0 "/Game/Materials/M_Yellow.M_Yellow"))))

(fn ConstructionScript)