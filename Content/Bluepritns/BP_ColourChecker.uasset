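; Puzzle checker that opens a door when colour switches match the required combination, triggered by a first-person projectile hitting its box.
; EvaluateColours compares each switch key's colour to its value in the ProperCombination map, tallying matches in SuccessCounter, which is never reset here.
; A full match shows confirmation text and plays the DoorOpening level sequence once through DoOnce; otherwise the text shows a random failure message.
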(event OnComponentHit(Box)
  (params (HitComponent :type Primitive%20Component%20Object%20Reference) (OtherActor :type Actor%20Object%20Reference) (OtherComp :type Primitive%20Component%20Object%20Reference) (NormalImpulse :type Vector :default "0, 0, 0") (Hit :type Hit%20Result%20Structure%20%28by%20ref%29))
  (if (== (Utilities|GetClass OtherActor) "/Game/FirstPerson/Blueprints/BP_FirstPersonProjectile.BP_FirstPersonProjectile_C")
    (CallFunction|EvaluateColours)))

(event EventBeginPlay
  (Variables|Default|SetMap%20Lenght (Utilities|Map|Length (Variables|Default|GetProper%20Combination)))
  (bind _returnvalue (Sequencer|Player|CreateLevelSequencePlayer "/Game/DoorOpening.DoorOpening"))
  (Variables|Default|SetSequence%20Player%20Reference _returnvalue))

(fn ConstructionScript)

(fn EvaluateColours
  (bind _proper_combination (Variables|Default|GetProper%20Combination))
  ;[1 1 1] Loop gets current Colour of a ColourSwitch, and compare it to a map variables adding Success Counters on positive comparison
  (for _index (range 0 (- (Variables|Default|GetMap%20Lenght) 1))
    (bind _keys (Utilities|Map|Keys _proper_combination))
    (if (== (.Value (Utilities|Map|Find _proper_combination (Utilities|Array|Get(acopy) _keys _index))) (Variables|/Game/Bluepritns/BP_ColourSwitch.BP_ColourSwitch_C|GetColour (Utilities|Array|Get(acopy) _keys _index)))
      (Math|Integer|IncrementInt (LocalVariables|GetSuccess%20Counter))))
  (if (== (LocalVariables|GetSuccess%20Counter) (Variables|Default|GetMap%20Lenght))
    (CallFunction|Success)
    (else
      (CallFunction|Failure))))

(fn Success
  (Rendering|Components|TextRender|SetText (Variables|Default|GetConfirmation%20Text) (Utilities|Text|ToText(String) (Utilities|String|Append "Correct Sequence" " 
" "You May Pass")))
  (Utilities|FlowControl|DoOnce false
    (:Completed
      (Sequencer|Player|Play (Variables|Default|GetSequence%20Player%20Reference) :!class /Script/MovieScene.MovieSceneSequencePlayer))))

(fn Failure
  (Rendering|Components|TextRender|SetText (Variables|Default|GetConfirmation%20Text) (Utilities|Text|ToText(String) (Utilities|String|Append (Utilities|Array|Get(acopy) (Variables|Default|GetList%20of%20Strings) (Math|Random|RandomIntegerinRange 0 10)) " 
" "Passage Closed"))))